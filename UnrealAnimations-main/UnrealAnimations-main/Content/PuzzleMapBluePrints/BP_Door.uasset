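; BP_Door is a puzzle-map door actor that opens by sliding upward and closes by returning to its start position.
; BeginPlay caches the start location and an end point offset vertically above it.
; OpenDoor spawns a confetti Niagara effect at an offset and plays the DoorMove timeline, lerping the location between both points without sweep.
; CloseDoor reverses that same timeline.
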(event `self.ReceiveBeginPlay`
  (bind _output_get (set `self.DoorStart` (`self.K2_GetActorLocation`)))
  (set `self.DoorEnd` (+ _output_get (0.0 0.0 400.0))))

(event `OpenDoor`
  (`NiagaraFunctionLibrary.SpawnSystemAtLocation` "/Game/PuzzleMapBluePrints/NS_Confetti.NS_Confetti" (+ (`self.K2_GetActorLocation`) (`self.ConfettiLocation`)))
  (bind (_direction _newtrack_0) (`Timeline|DoorMove` :!label _label)
    (:`Update`
      (`self.K2_SetActorLocation` (`KismetMathLibrary.VLerp` (`self.DoorStart`) (`self.DoorEnd`) _newtrack_0)))))

(event `CloseDoor`
  (goto _label :!via `Reverse`))

(fn `UserConstructionScript`)